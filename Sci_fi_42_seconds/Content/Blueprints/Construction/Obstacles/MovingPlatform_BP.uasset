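; MovingPlatform_BP is an obstacle platform that shuttles a Cube back and forth between StartPoint and EndPoint, starting on BeginPlay.
; The Movement timeline lerps the Cube's relative location forward, and a second timeline, Timeline_0, plays in reverse to bring it back.
; Each timeline's finish triggers the other after a short delay, forming an endless loop with no sweep on movement.
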(event `self.ReceiveBeginPlay`
  (bind (_direction _newtrack_0) (`Timeline|Movement` :!label _label)
    (:`Update`
      (`SceneComponent.K2_SetRelativeLocation` (`self.Cube`) (`KismetMathLibrary.VLerp` (`SceneComponent.RelativeLocation` (`self.Start point`)) (`SceneComponent.RelativeLocation` (`self.End point`)) _newtrack_0) false false))
    (:`Finished`
      (`KismetSystemLibrary.Delay` 0.3)
      (bind (_direction_2 _newtrack_0_2) (`Timeline|Timeline_0` :!via `ReverseFromEnd`)
        (:`Update`
          (`SceneComponent.K2_SetRelativeLocation` (`self.Cube`) (`KismetMathLibrary.VLerp` (`SceneComponent.RelativeLocation` (`self.Start point`)) (`SceneComponent.RelativeLocation` (`self.End point`)) _newtrack_0_2) false false))
        (:`Finished`
          (`KismetSystemLibrary.Delay` 0.3)
          (goto _label :!via `PlayFromStart`))))))

(fn `UserConstructionScript`)