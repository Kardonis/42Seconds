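; On_Off_Button_BP is an obstacle button that toggles the game-wide on/off block state.
; Each overlap with its Box flips AreBlocksOn on ThirdPersonGameMode, swaps the Sphere material between red (on) and cyan (off), and plays a click sound.
; The cached player-character comparison is disconnected, so the toggle does not filter which actor overlaps it.
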(event `self.ReceiveBeginPlay`
  (bind _asthird_person_game_mode (cast `/Game/GameModes/ThirdPersonGameMode` (`GameplayStatics.GetGameMode`)))
  (set `self.GameMode` _asthird_person_game_mode)
  (bind _asthird_person_character (cast `/Game/Character/ThirdPersonCharacter` (`GameplayStatics.GetPlayerCharacter` 0)))
  (set `self.PlayerCharacter` _asthird_person_character))

(event `self.Box.OnComponentBeginOverlap`
  (params (OverlappedComponent :type "PrimitiveComponent Object Reference") (OtherActor :type "Actor Object Reference") (OtherComp :type "PrimitiveComponent Object Reference") (OtherBodyIndex :type Integer) (bFromSweep :type Boolean) (SweepResult :type "HitResult Structure (by ref)"))
  (bind _gamemode (`self.GameMode`))
  (bind _sphere (`self.Sphere`))
  (if (`/Game/GameModes/ThirdPersonGameMode.AreBlocksOn?` _gamemode)
    (set `/Game/GameModes/ThirdPersonGameMode.AreBlocksOn?` false _gamemode)
    (`PrimitiveComponent.SetMaterial` _sphere 0 "/Game/Blueprints/TempMaterials/Cyan.Cyan")
    (else
      (set `/Game/GameModes/ThirdPersonGameMode.AreBlocksOn?` true _gamemode)
      (`PrimitiveComponent.SetMaterial` _sphere 0 "/Game/Blueprints/TempMaterials/Red.Red")))
  (`GameplayStatics.SpawnSoundAtLocation` "/Game/Audio/click.Click" (`self.K2_GetActorLocation`) (struct) 1.0 1.0 0.0 null null))

(fn `UserConstructionScript`)