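; Start elevator Blueprint that raises itself 600 units from its placed position when play begins.
; BeginPlay stores start and end points, then the ElevatorArriving timeline lerps the root component's relative location between them.
; The Entry overlap event is empty.
; Disconnected nodes would cache the character and game mode, and, for the player, stop the timer, disable input and play an ElevatorLeaving timeline, but they never run.
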(event `self.ReceiveBeginPlay`
  (set `self.StartPoint` (`SceneComponent.RelativeLocation` (`self.DefaultSceneRoot`)))
  (set `self.EndPoint` (+ (`self.StartPoint`) (0.0 0.0 600.0)))
  (bind (_direction _newtrack_0) (`Timeline|Elevator Arriving`)
    (:`Update`
      (`SceneComponent.K2_SetRelativeLocation` (`self.DefaultSceneRoot`) (`KismetMathLibrary.VLerp` (`self.StartPoint`) (`self.EndPoint`) _newtrack_0) false false))))

(event `self.Entry.OnComponentBeginOverlap`
  (params (OverlappedComponent :type "PrimitiveComponent Object Reference") (OtherActor :type "Actor Object Reference") (OtherComp :type "PrimitiveComponent Object Reference") (OtherBodyIndex :type Integer) (bFromSweep :type Boolean) (SweepResult :type "HitResult Structure (by ref)")))

(fn `UserConstructionScript`)