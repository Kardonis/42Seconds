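; LightGate_BP is a gate actor that sends the player into a portal on contact.
; On BeginPlay it caches the ThirdPersonCharacter and the ThirdPersonGameMode, though the game mode is not used afterwards.
; When the cached player begins overlapping the Entry component, the gate calls EnterPortal with true on that character, which owns the portal behavior.
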(event `self.ReceiveBeginPlay`
  ;[1 1 1] Setup
  (bind _asthird_person_character (cast `/Game/Character/ThirdPersonCharacter` (`GameplayStatics.GetPlayerCharacter` 0)))
  (set `self.PlayerCharacter` _asthird_person_character)
  (bind _asthird_person_game_mode (cast `/Game/GameModes/ThirdPersonGameMode` (`GameplayStatics.GetGameMode`)))
  (set `self.GameMode` _asthird_person_game_mode))

(event `self.Entry.OnComponentBeginOverlap`
  (params (OverlappedComponent :type "PrimitiveComponent Object Reference") (OtherActor :type "Actor Object Reference") (OtherComp :type "PrimitiveComponent Object Reference") (OtherBodyIndex :type Integer) (bFromSweep :type Boolean) (SweepResult :type "HitResult Structure (by ref)"))
  (if (== (`self.PlayerCharacter`) OtherActor)
    (`/Game/Character/ThirdPersonCharacter.EnterPortal` (`self.PlayerCharacter`) true)))

(fn `UserConstructionScript`)