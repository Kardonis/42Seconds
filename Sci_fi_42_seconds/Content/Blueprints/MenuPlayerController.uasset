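; Player controller for the menu that lets the mouse wheel zoom the world map widget.
; BeginPlay caches the MenuGameMode and calls Possess with no pawn specified.
; Tick polls the game mode's IsMapActive flag, grabbing the first top-level World_Map widget when active and clearing it when inactive.
; While the map is active, wheel presses resize that widget by a fixed percentage, with debug prints throughout.
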(event `self.ReceiveBeginPlay`
  (bind _asmenu_game_mode (cast `/Game/GameModes/MenuGameMode` (`GameplayStatics.GetGameMode`)))
  (set `self.GameMode` _asmenu_game_mode)
  (`self.Possess` null)
  (`KismetSystemLibrary.PrintString` "whee"))

(event `self.ReceiveTick`
  (params (DeltaSeconds :type "Float (single-precision)"))
  (bind _ismapactive_ (`/Game/GameModes/MenuGameMode.IsMapActive?` (`self.GameMode`)))
  (if (`self.IsMapSet?`)
    (if (not _ismapactive_)
      (set `self.WorldMap` null)
      (bind _output_get (set `self.IsMapSet?` false))
      (`KismetSystemLibrary.PrintString` (`KismetStringLibrary.Conv_BoolToString` _output_get)))
    (elif _ismapactive_
      (bind _foundwidgets (`WidgetBlueprintLibrary.GetAllWidgetsOfClass` "/Game/UI/MenuUI/World_Map.World_Map_C"))
      (set `self.WorldMap` (`|GetArrayItem` _foundwidgets))
      (set `self.IsMapSet?` true)
      (`KismetSystemLibrary.PrintString` "Hello"))))

(event `Key|MouseScrollUp` :paused true
  (params (Key :type "Key Structure"))
  (:`Pressed`
    (if (`/Game/GameModes/MenuGameMode.IsMapActive?` (`self.GameMode`))
      (`/Game/UI/MenuUI/World_Map.OutputModifySize` (`self.WorldMap`) true 10)
      (`KismetSystemLibrary.PrintString` "Hello" :!label _label)
      (else
        (`KismetSystemLibrary.PrintString` "map not active" :!label _label_2)))))

(event `Key|MouseScrollDown` :paused true
  (params (Key :type "Key Structure"))
  (:`Pressed`
    (if (`/Game/GameModes/MenuGameMode.IsMapActive?` (`self.GameMode`))
      (`/Game/UI/MenuUI/World_Map.OutputModifySize` (`self.WorldMap`) false 10)
      (goto _label)
      (else
        (goto _label_2)))))

(fn `UserConstructionScript`)