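; On/off platform obstacle that appears and disappears based on a shared switch in the game mode.
; BeginPlay caches the ThirdPersonGameMode.
; Each Tick polls its AreBlocksOn flag, showing the Platform with full query and physics collision when true, or hiding it with no collision when false.
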(event `self.ReceiveBeginPlay`
  (bind _asthird_person_game_mode (cast `/Game/GameModes/ThirdPersonGameMode` (`GameplayStatics.GetGameMode`)))
  (set `self.GameMode` _asthird_person_game_mode))

(event `self.ReceiveTick`
  (params (DeltaSeconds :type "Float (single-precision)"))
  (bind _platform (`self.Platform`))
  (if (`/Game/GameModes/ThirdPersonGameMode.AreBlocksOn?` (`self.GameMode`))
    (`SceneComponent.SetVisibility` _platform true false)
    (`PrimitiveComponent.SetCollisionEnabled` _platform "QueryAndPhysics")
    (else
      (`SceneComponent.SetVisibility` _platform false false)
      (`PrimitiveComponent.SetCollisionEnabled` _platform "NoCollision"))))

(fn `UserConstructionScript`)