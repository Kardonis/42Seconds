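; VoidGate_BP is a portal gate that stops the game timer and sends the player into the portal on contact.
; BeginPlay caches the player's ThirdPersonCharacter and the ThirdPersonGameMode.
; When that character overlaps the Entry component, the gate plays a 2D whoosh sound, clears the game mode's IsTimerRunning flag and calls EnterPortal on the character.
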(event `self.ReceiveBeginPlay`
  ;[1 1 1] Setup
  (bind _asthird_person_character (cast `/Game/Character/ThirdPersonCharacter` (`GameplayStatics.GetPlayerCharacter` 0)))
  (set `self.PlayerCharacter` _asthird_person_character)
  (bind _asthird_person_game_mode (cast `/Game/GameModes/ThirdPersonGameMode` (`GameplayStatics.GetGameMode`)))
  (set `self.GameMode` _asthird_person_game_mode))

(event `self.Entry.OnComponentBeginOverlap`
  (params (OverlappedComponent :type "PrimitiveComponent Object Reference") (OtherActor :type "Actor Object Reference") (OtherComp :type "PrimitiveComponent Object Reference") (OtherBodyIndex :type Integer) (bFromSweep :type Boolean) (SweepResult :type "HitResult Structure (by ref)"))
  (if (== (`self.PlayerCharacter`) OtherActor)
    (`GameplayStatics.PlaySound2D` "/Game/Audio/Woosh_but_better.Woosh_but_better" 1.25 1.0 1.1 null null)
    (set `/Game/GameModes/ThirdPersonGameMode.IsTimerRunning?` false (`self.GameMode`))
    (`/Game/Character/ThirdPersonCharacter.EnterPortal` (`self.PlayerCharacter`) true)))

(fn `UserConstructionScript`)