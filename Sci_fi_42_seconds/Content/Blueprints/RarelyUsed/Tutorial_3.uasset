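; Tutorial trigger Blueprint that shows a sprint tutorial widget while the player is inside its box.
; BeginPlay caches the player character, and a box begin overlap by that character creates the Tutorial_Sprint widget and adds it to the viewport.
; End overlap removes the widget without checking which actor left.
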(event `self.ReceiveBeginPlay`
  (set `self.Player` (`GameplayStatics.GetPlayerCharacter` 0)))

(event `self.Box.OnComponentBeginOverlap`
  (params (OverlappedComponent :type "PrimitiveComponent Object Reference") (OtherActor :type "Actor Object Reference") (OtherComp :type "PrimitiveComponent Object Reference") (OtherBodyIndex :type Integer) (bFromSweep :type Boolean) (SweepResult :type "HitResult Structure (by ref)"))
  (if (== OtherActor (`self.Player`))
    (bind _returnvalue (`|CreateWidget` "/Game/UI/GamePlayUI/Tutorials/Tutorial_Sprint.Tutorial_Sprint_C" (`GameplayStatics.GetPlayerController` 0)))
    (`UserWidget.AddToViewport` _returnvalue 0)))

(event `self.Box.OnComponentEndOverlap`
  (params (OverlappedComponent :type "PrimitiveComponent Object Reference") (OtherActor :type "Actor Object Reference") (OtherComp :type "PrimitiveComponent Object Reference") (OtherBodyIndex :type Integer))
  (`Widget.RemoveFromParent` (stale `self.Box.OnComponentBeginOverlap` _returnvalue)))

(fn `UserConstructionScript`)