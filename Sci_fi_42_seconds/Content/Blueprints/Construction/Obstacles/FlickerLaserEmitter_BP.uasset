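; Laser obstacle that flickers on and off and destroys the player on contact while active.
; BeginPlay caches the player character, then runs an endless Delay loop that sets the particle beam between two emitter components and toggles it with the Active flag.
; Capsule begin-overlap calls the player's Destroyed only while Active, so a player already inside when the beam reactivates is not caught.
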(event `self.ReceiveBeginPlay`
  (bind _asthird_person_character (cast `/Game/Character/ThirdPersonCharacter` (`GameplayStatics.GetPlayerCharacter` 0)))
  (set `self.Player` _asthird_person_character)
  (`ParticleSystemComponent.SetBeamSourcePoint` (`self.ParticleSystem`) 0 (`SceneComponent.K2_GetComponentLocation` (`self.Emitter`)) 0 :!label _label)
  (`ParticleSystemComponent.SetBeamEndPoint` (`self.ParticleSystem`) 0 (`SceneComponent.K2_GetComponentLocation` (`self.Emitter_2`)))
  (`KismetSystemLibrary.Delay` 2.0)
  (`ActorComponent.Deactivate` (`self.ParticleSystem`))
  (set `self.Active` false)
  (`KismetSystemLibrary.Delay` 3.0)
  (`ActorComponent.Activate` (`self.ParticleSystem`) false)
  (set `self.Active` true)
  (goto _label))

(event `self.Capsule.OnComponentBeginOverlap`
  (params (OverlappedComponent :type "PrimitiveComponent Object Reference") (OtherActor :type "Actor Object Reference") (OtherComp :type "PrimitiveComponent Object Reference") (OtherBodyIndex :type Integer) (bFromSweep :type Boolean) (SweepResult :type "HitResult Structure (by ref)"))
  (bind _player (`self.Player`))
  (if (`self.Active`)
    (if (== OtherActor _player)
      (`/Game/Character/ThirdPersonCharacter.Destroyed` _player true))))

(fn `UserConstructionScript`)