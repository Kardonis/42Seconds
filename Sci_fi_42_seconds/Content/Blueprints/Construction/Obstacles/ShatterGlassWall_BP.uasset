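; Breakable glass wall obstacle that shatters when the player runs into it fast enough.
; On BeginPlay it caches the player's ThirdPersonCharacter, and the Box1 overlap responds only to that actor.
; If any single velocity axis reaches the speed threshold in either direction, it plays a 2D shatter sound and destroys itself.
; The check is per world axis rather than on overall speed, and no debris is spawned.
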(event `self.ReceiveBeginPlay`
  (bind _asthird_person_character (cast `/Game/Character/ThirdPersonCharacter` (`GameplayStatics.GetPlayerCharacter` 0)))
  (set `self.Player` _asthird_person_character))

(event `self.Box1.OnComponentBeginOverlap`
  (params (OverlappedComponent :type "PrimitiveComponent Object Reference") (OtherActor :type "Actor Object Reference") (OtherComp :type "PrimitiveComponent Object Reference") (OtherBodyIndex :type Integer) (bFromSweep :type Boolean) (SweepResult :type "HitResult Structure (by ref)"))
  (bind _player (`self.Player`))
  (bind _x (.x (`self.GetVelocity` _player)))
  (bind _y (.y (`self.GetVelocity` _player)))
  (bind _z (.z (`self.GetVelocity` _player)))
  (if (== OtherActor _player)
    (if (or (or (>= _x 800.0) (>= _y 800.0) (>= _z 800.0)) (or (<= _x -800.0) (<= _y -800.0) (<= _z -800.0)))
      (`GameplayStatics.SpawnSound2D` "/Game/Audio/Glass_Shatter.Glass_Shatter" 1.0 1.0 0.2 null)
      (`self.K2_DestroyActor`))))

(fn `UserConstructionScript`)