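; Final exit elevator that ends the run when the player enters its Entry trigger.
; On overlap it stops the GameMode timer and calls Completed on the character as a final exit with bonus.
; A timeline turns the character toward the Arrow while also rotating its camera boom, then a second timeline lifts the elevator's root component to a fixed height above its start.
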(event `self.ReceiveBeginPlay`
  ;[1 1 1] Setup
  (bind _asthird_person_character (cast `/Game/Character/ThirdPersonCharacter` (`GameplayStatics.GetPlayerCharacter` 0)))
  (set `self.PlayerCharacter` _asthird_person_character)
  (bind _asthird_person_game_mode (cast `/Game/GameModes/ThirdPersonGameMode` (`GameplayStatics.GetGameMode`)))
  (set `self.GameMode` _asthird_person_game_mode)
  (set `self.StartPoint` (`SceneComponent.RelativeLocation` (`self.DefaultSceneRoot`)))
  (set `self.EndPoint` (+ (`self.StartPoint`) (0.0 0.0 600.0))))

(event `self.Entry.OnComponentBeginOverlap`
  (params (OverlappedComponent :type "PrimitiveComponent Object Reference") (OtherActor :type "Actor Object Reference") (OtherComp :type "PrimitiveComponent Object Reference") (OtherBodyIndex :type Integer) (bFromSweep :type Boolean) (SweepResult :type "HitResult Structure (by ref)"))
  (bind _playercharacter (`self.PlayerCharacter`))
  (if (== (`self.PlayerCharacter`) OtherActor)
    (set `/Game/GameModes/ThirdPersonGameMode.IsTimerRunning?` false (`self.GameMode`))
    (`/Game/Character/ThirdPersonCharacter.Completed` _playercharacter true true false)
    (bind _output_get (set `self.PlayerRotation` (`SceneComponent.K2_GetComponentRotation` (`Character.CapsuleComponent` _playercharacter))))
    (bind (_direction _newtrack_0) (`Timeline|Timeline_0`)
      (:`Update`
        (bind _returnvalue (`KismetMathLibrary.RLerp` _output_get (`SceneComponent.K2_GetComponentRotation` (`self.Arrow`)) _newtrack_0 true))
        (`self.K2_SetActorRelativeRotation` (`self.PlayerCharacter`) _returnvalue false false)
        (`SceneComponent.K2_AddWorldRotation` (`/Game/Character/ThirdPersonCharacter.CameraBoom` (`self.PlayerCharacter`)) _returnvalue false false))
      (:`Finished`
        (bind (_direction_2 _newtrack_0_2) (`Timeline|ElevatorLeaving`)
          (:`Update`
            (`SceneComponent.K2_SetRelativeLocation` (`self.DefaultSceneRoot`) (`KismetMathLibrary.VLerp` (`self.StartPoint`) (`self.EndPoint`) _newtrack_0_2) false false)))))))

(fn `UserConstructionScript`)