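; Secret_BP is a collectible secret pickup that shows a spinning Chip component.
; The Chip rotates by a fixed step every Tick, independent of delta time.
; When the player character cached at BeginPlay overlaps the Sphere, it sets SecretFound on the ThirdPersonCharacter and destroys itself.
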(event `self.ReceiveBeginPlay`
  (set `self.Player` (`GameplayStatics.GetPlayerCharacter` 0)))

(event `self.ReceiveTick`
  (params (DeltaSeconds :type "Float (single-precision)"))
  (`SceneComponent.K2_AddRelativeRotation` (`self.Chip`) (struct :`Yaw` 1.0) false false))

(event `self.Sphere.OnComponentBeginOverlap`
  (params (OverlappedComponent :type "PrimitiveComponent Object Reference") (OtherActor :type "Actor Object Reference") (OtherComp :type "PrimitiveComponent Object Reference") (OtherBodyIndex :type Integer) (bFromSweep :type Boolean) (SweepResult :type "HitResult Structure (by ref)"))
  (if (== OtherActor (`self.Player`))
    (bind _asthird_person_character (cast `/Game/Character/ThirdPersonCharacter` (`self.Player`)))
    (set `/Game/Character/ThirdPersonCharacter.SecretFound` true _asthird_person_character)
    (`self.K2_DestroyActor`)))

(fn `UserConstructionScript`)