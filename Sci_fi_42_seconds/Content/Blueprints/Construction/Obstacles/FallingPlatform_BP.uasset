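; FallingPlatform_BP is an obstacle platform that drops shortly after the player touches it and then removes itself.
; On BeginPlay it caches the player's ThirdPersonCharacter, and the Box overlap responds only to that actor.
; After a short delay, the Movement timeline lerps the Cube's relative location from StartPoint to EndPoint without sweep, then destroys the actor when finished.
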(event `self.ReceiveBeginPlay`
  (bind _asthird_person_character (cast `/Game/Character/ThirdPersonCharacter` (`GameplayStatics.GetPlayerCharacter` 0)))
  (set `self.player` _asthird_person_character))

(event `self.Box.OnComponentBeginOverlap`
  (params (OverlappedComponent :type "PrimitiveComponent Object Reference") (OtherActor :type "Actor Object Reference") (OtherComp :type "PrimitiveComponent Object Reference") (OtherBodyIndex :type Integer) (bFromSweep :type Boolean) (SweepResult :type "HitResult Structure (by ref)"))
  (if (== OtherActor (`self.player`))
    (`KismetSystemLibrary.Delay` 0.5)
    (bind (_direction _newtrack_0) (`Timeline|Movement`)
      (:`Update`
        (`SceneComponent.K2_SetRelativeLocation` (`self.Cube`) (`KismetMathLibrary.VLerp` (`SceneComponent.RelativeLocation` (`self.Start point`)) (`SceneComponent.RelativeLocation` (`self.End point`)) _newtrack_0) false false))
      (:`Finished`
        (`self.K2_DestroyActor`)))))

(fn `UserConstructionScript`)